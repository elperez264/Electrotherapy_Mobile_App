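; RoundSlider is a rotary slider actor that raises or lowers a power value and turns a wheel to match.
; Increase and Decrease events read the power from Value, check it against an upper or lower limit, then yaw the Wheel one fixed step and forward the change to Value.
; Nothing in its own graph calls these events, and BeginPlay, overlap and Tick are unused.
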(event `/Game/AppContent/Interface/SliderInterface.Increase`
  (bind _wheel (`self.Wheel`))
  (bind (_relativerotation_roll _relativerotation_pitch _relativerotation_yaw) (`KismetMathLibrary.BreakRotator` (`SceneComponent.RelativeRotation` _wheel)))
  (bind _value (`/Game/AppContent/Blueprints/Power_Indicator.GetPower` (`self.Value`)))
  (if (< _value 349)
    (`SceneComponent.K2_SetRelativeRotation` _wheel (`KismetMathLibrary.MakeRotator` 0.0 0.0 (+ _relativerotation_yaw 4.0)) false false)
    (`/Game/AppContent/Blueprints/Power_Indicator.Increase` (`self.Value`))))

(event `/Game/AppContent/Interface/SliderInterface.Decrease`
  (bind _wheel (`self.Wheel`))
  (bind (_relativerotation_roll _relativerotation_pitch _relativerotation_yaw) (`KismetMathLibrary.BreakRotator` (`SceneComponent.RelativeRotation` _wheel)))
  (bind _value (`/Game/AppContent/Blueprints/Power_Indicator.GetPower` (`self.Value`)))
  (if (> _value 1)
    (`SceneComponent.K2_SetRelativeRotation` _wheel (`KismetMathLibrary.MakeRotator` 0.0 0.0 (+ _relativerotation_yaw -4.0)) false false)
    (`/Game/AppContent/Blueprints/Power_Indicator.Decrease` (`self.Value`))))

(fn `UserConstructionScript`)