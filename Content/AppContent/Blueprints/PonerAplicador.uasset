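; PonerAplicador is a pressable button actor that toggles placing and removing an applicator through a Manager reference.
; Press nudges the Cube down and, after a short delay, restores it, then calls Aplicar or Quitar depending on the Aplicated flag.
; Applying always sets the flag, while removal clears it only if Quitar succeeds.
; The TextRender label switches between the Spanish put and remove captions with each state change.
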(event `/Game/AppContent/Interface/ButtonInterface.Press`
  (bind _manager (`self.Manager`))
  (`SceneComponent.K2_SetRelativeLocation` (`self.Cube`) (0.0 0.0 -20.0) false false)
  (`KismetSystemLibrary.Delay` 0.2)
  (`SceneComponent.K2_SetRelativeLocation` (`self.Cube`) (0.0 0.0 0.0) false false)
  (if (`self.Aplicated`)
    (bind _removewell (`/Game/AppContent/Blueprints/NotificationManager.Quitar` _manager))
    (if _removewell
      (set `self.Aplicated` false)
      (`TextRenderComponent.K2_SetText` (`self.TextRender`) (`|FormatText` "Poner aplicador")))
    (else
      (`/Game/AppContent/Blueprints/NotificationManager.Aplicar` _manager)
      (set `self.Aplicated` true)
      (`TextRenderComponent.K2_SetText` (`self.TextRender`) (`|FormatText` "Quitar aplicador")))))

(fn `UserConstructionScript`)