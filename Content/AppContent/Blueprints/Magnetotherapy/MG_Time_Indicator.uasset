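; Time indicator for the magnetotherapy app that holds a duration in seconds and shows it on a TimeNumber widget.
; Increase and Decrease step the value by one within max and min limits, updating the widget's Hours and Minutes inputs with minutes and seconds.
; TimeDown counts down one second per call, ignoring the minimum, and calls FinishTimer on Pantalla when called at zero.
; PowerOff is an empty stub.
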(event `self.PowerOff`)

(event `self.Decrease`
  (bind _yes (`self.isMin`))
  (if (not _yes)
    (`self.DecreaseTime`)))

(event `self.Increase`
  (bind _yes (`self.isMax`))
  (if (not _yes)
    (bind _output_get (set `self.ValueSeconds` (+ (`self.ValueSeconds`) 1)))
    (bind _astime_number (cast `/Game/AppContent/UI/TimeNumber` (`WidgetComponent.GetUserWidgetObject` (`self.Widget`))))
    (`/Game/AppContent/UI/TimeNumber.SetValue_Event` _astime_number (/ _output_get 60) (mod _output_get 60))))

(fn `DecreaseTime`
  (bind _output_get (set `self.ValueSeconds` (- (`self.ValueSeconds`) 1)))
  (bind _astime_number (cast `/Game/AppContent/UI/TimeNumber` (`WidgetComponent.GetUserWidgetObject` (`self.Widget`))))
  (`/Game/AppContent/UI/TimeNumber.SetValue_Event` _astime_number (/ _output_get 60) (mod _output_get 60)))

(fn `IsLessThanMin`
  (returns (yes :type Boolean))
  (return (< (`self.ValueSeconds`) (`self.MinValue`))))

(fn `isMax`
  (returns (yes :type Boolean))
  (return (>= (`self.ValueSeconds`) (`self.MaxValue`))))

(fn `isMin`
  (returns (yes :type Boolean))
  (return (<= (`self.ValueSeconds`) (`self.MinValue`))))

(fn `TimeDown`
  (if (>= (`self.ValueSeconds`) 1)
    (`self.DecreaseTime`)
    (else
      (`/Game/AppContent/Blueprints/Magnetotherapy/PantallaMagneto.FinishTimer` (`self.Pantalla`)))))

(fn `UserConstructionScript`)