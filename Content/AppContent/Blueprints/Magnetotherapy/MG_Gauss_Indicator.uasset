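; MG_Gauss_Indicator is the Gauss value display for the magnetotherapy device, showing its setting through a GaussNumber widget.
; Increase and Decrease step the value by a fixed amount while powered on and not counting down, with checks against the minimum and maximum.
; Each change is pushed to the widget via SetValueEvent.
; PowerOn only sets the on flag, while PowerOff resets the value and display to the minimum.
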(event `self.PowerOff`
  (set `self.Value` (`self.MinValue`))
  (bind _asgauss_number (cast `/Game/AppContent/UI/GaussNumber` (`WidgetComponent.GetUserWidgetObject` (`self.Widget`))))
  (`/Game/AppContent/UI/GaussNumber.SetValue_Event` _asgauss_number (`self.MinValue`))
  (set `self.isOn` false))

(event `self.Decrease`
  (if (and (`self.isOn`) (not (`self.isCountingDown`)))
    (bind _yes (`self.isMin`))
    (if (not _yes)
      (bind _output_get (set `self.Value` (- (`self.Value`) 5)))
      (bind _asgauss_number (cast `/Game/AppContent/UI/GaussNumber` (`WidgetComponent.GetUserWidgetObject` (`self.Widget`))))
      (`/Game/AppContent/UI/GaussNumber.SetValue_Event` _asgauss_number _output_get))))

(event `self.Increase`
  (if (and (`self.isOn`) (not (`self.isCountingDown`)))
    (bind _yes (`self.isMax`))
    (if (not _yes)
      (bind _output_get (set `self.Value` (+ (`self.Value`) 5)))
      (bind _asgauss_number (cast `/Game/AppContent/UI/GaussNumber` (`WidgetComponent.GetUserWidgetObject` (`self.Widget`))))
      (`/Game/AppContent/UI/GaussNumber.SetValue_Event` _asgauss_number _output_get))))

(fn `isMax`
  (returns (yes :type Boolean))
  (return (>= (`self.Value`) (`self.MaxValue`))))

(fn `isMin`
  (returns (yes :type Boolean))
  (return (<= (`self.Value`) (`self.MinValue`))))

(fn `PowerOn`
  (set `self.isOn` true))

(fn `UserConstructionScript`)