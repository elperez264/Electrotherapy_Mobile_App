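; MG_Hz_Indicator is the frequency (Hz) indicator actor for the magnetotherapy device, holding the current value and showing it on a widget.
; Increase and Decrease events step the value by one, guarded by IsMax and IsMin checks against the configured limits.
; Each change is pushed to the HzNumber user widget through its SetValueEvent.
; The PowerOff event is an empty stub.
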(event `self.PowerOff`)

(event `self.Decrease`
  (bind _yes (`self.isMin`))
  (if (not _yes)
    (bind _output_get (set `self.Value` (- (`self.Value`) 1)))
    (bind _ashz_number (cast `/Game/AppContent/UI/HzNumber` (`WidgetComponent.GetUserWidgetObject` (`self.Widget`))))
    (`/Game/AppContent/UI/HzNumber.SetValue_Event` _ashz_number _output_get)))

(event `self.Increase`
  (bind _yes (`self.isMax`))
  (if (not _yes)
    (bind _output_get (set `self.Value` (+ (`self.Value`) 1)))
    (bind _ashz_number (cast `/Game/AppContent/UI/HzNumber` (`WidgetComponent.GetUserWidgetObject` (`self.Widget`))))
    (`/Game/AppContent/UI/HzNumber.SetValue_Event` _ashz_number _output_get)))

(fn `isMax`
  (returns (yes :type Boolean))
  (return (>= (`self.Value`) (`self.MaxValue`))))

(fn `isMin`
  (returns (yes :type Boolean))
  (return (<= (`self.Value`) (`self.MinValue`))))

(fn `UserConstructionScript`)