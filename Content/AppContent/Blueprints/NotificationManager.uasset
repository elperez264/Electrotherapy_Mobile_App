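; Notification manager actor that gives right-or-wrong feedback on the order in which an applicator is applied or removed and a machine is started or switched off.
; It adds a Notifications widget to the viewport on BeginPlay and tracks applicator placement in Aplicado.
; Each action function checks that flag or the countdown state from Tiempo.
; Start and shutdown trigger widget events, while applicator changes only print Spanish messages.
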(event `self.ReceiveBeginPlay`
  (bind _returnvalue (`|CreateWidget` "/Game/AppContent/UI/Notifications.Notifications_C" (`GameplayStatics.GetPlayerController` 0)))
  (bind _output_get (set `self.UI` _returnvalue))
  (`UserWidget.AddToViewport` _output_get 0))

(fn `Apagar`
  (params (isCountingDown :type Boolean))
  (if (and isCountingDown (`self.Aplicado`))
    (`/Game/AppContent/UI/Notifications.Mal_Apagar_Event` (`self.UI`))))

(fn `Aplicar`
  ;[0.04167 0.04167 0.04167] Si tengo una notificacion de que ha empezado sin el aplicador este mensaje sobra
  (set `self.Aplicado` true)
  (bind _countdown (`/Game/AppContent/Blueprints/Time_Indicator.IsCountingDown` (`self.Tiempo`)))
  (if _countdown
    (`KismetSystemLibrary.PrintString` "Deberias colocar el aplicador antes de empezar")))

(fn `Empezar`
  (bind _ui (`self.UI`))
  (bind _countdown (`/Game/AppContent/Blueprints/Time_Indicator.IsCountingDown` (`self.Tiempo`)))
  (if _countdown
    (if (`self.Aplicado`)
      (`/Game/AppContent/UI/Notifications.Bien_comenzar_Event` _ui)
      (else
        (`/Game/AppContent/UI/Notifications.Mal_Comenzar_Event` _ui)))))

(fn `Quitar`
  (set `self.Aplicado` false)
  (bind _countdown (`/Game/AppContent/Blueprints/Time_Indicator.IsCountingDown` (`self.Tiempo`)))
  (if _countdown
    (`KismetSystemLibrary.PrintString` "Tienes que apagar antes la maquina")
    (else
      (`KismetSystemLibrary.PrintString` "Bien"))))

(fn `UserConstructionScript`)