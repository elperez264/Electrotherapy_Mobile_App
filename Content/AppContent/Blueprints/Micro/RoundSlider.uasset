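; RoundSlider is a rotary dial actor that steps a time or power indicator up and down.
; Increase and Decrease yaw the Wheel by a fixed step and forward the change to the active indicator, stopping at that indicator's limits.
; SetIndicator switches the active indicator by Spanish name (Tiempo or Potencia), with time selected at BeginPlay.
; The wheel's rotation is not adjusted when the indicator switches.
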(event `self.ReceiveBeginPlay`
  (set `self.Value` (`self.TImeInd`)))

(event `/Game/AppContent/Interface/SliderInterface.Increase`
  (bind _wheel (`self.Wheel`))
  (bind (_relativerotation_roll _relativerotation_pitch _relativerotation_yaw) (`KismetMathLibrary.BreakRotator` (`SceneComponent.RelativeRotation` _wheel)))
  (bind _yes (`/Game/AppContent/Interface/IndicatorInterface.isMax` (`self.Value`)))
  (if (not _yes)
    (`SceneComponent.K2_SetRelativeRotation` _wheel (`KismetMathLibrary.MakeRotator` 0.0 0.0 (+ _relativerotation_yaw 4.0)) false false)
    (`/Game/AppContent/Interface/IndicatorInterface.Increase` (`self.Value`))))

(event `/Game/AppContent/Interface/SliderInterface.Decrease`
  (bind _wheel (`self.Wheel`))
  (bind (_relativerotation_roll _relativerotation_pitch _relativerotation_yaw) (`KismetMathLibrary.BreakRotator` (`SceneComponent.RelativeRotation` _wheel)))
  (bind _yes (`/Game/AppContent/Interface/IndicatorInterface.isMin` (`self.Value`)))
  (if (not _yes)
    (`SceneComponent.K2_SetRelativeRotation` _wheel (`KismetMathLibrary.MakeRotator` 0.0 0.0 (+ _relativerotation_yaw -4.0)) false false)
    (`/Game/AppContent/Interface/IndicatorInterface.Decrease` (`self.Value`))))

(fn `SetIndicator`
  (params (NameIndicator :type Text))
  (switch `string` (`KismetTextLibrary.Conv_TextToString` NameIndicator)
    (:`Tiempo`
      (set `self.Value` (`self.TImeInd`)))
    (:`Potencia`
      (set `self.Value` (`self.PowerInd`)))))

(fn `UserConstructionScript`)