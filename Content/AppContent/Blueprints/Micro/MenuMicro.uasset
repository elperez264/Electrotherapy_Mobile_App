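; Screen menu controller for the Micro device, showing options on a TextRender and handling power state.
; A menu selector cycles entries or returns from the applicator and emission submenus, pointing the Wheel at Tiempo (time) or Potencia (power) when shown.
; Enter opens submenus, toggles the Time countdown on Comenzar (start), or advances otherwise.
; Countdown state is mirrored to Power and locks navigation; powering off hides and resets the screen.
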(event `self.ReceiveBeginPlay`
  (set `self.ActualMenu` (`self.MainMenu`)))

(event `/Game/AppContent/Interface/PantallaMenu.Enter`
  (bind _time (`self.Time`))
  (if (`self.Encendido`)
    (switch `string` (`KismetTextLibrary.Conv_TextToString` (`|GetArrayItem` (`self.ActualMenu`) (`self.index`)))
      (:`Default`
        (`self.ChangeMenu`))
      (:`Tipo de Aplicador`
        ;[0.0625 0.0625 0.0625] Set the submenus
        (bind _output_get (set `self.ActualMenu` (`self.AplicadorMenu`)))
        (`TextRenderComponent.K2_SetText` (`self.TextRender`) (`|GetArrayItem` _output_get))
        (set `self.isInSubmenu` true :!label _label)
        (set `self.index` 0))
      (:`Tipo de Emision`
        (bind _output_get_2 (set `self.ActualMenu` (`self.EmisionMenu`)))
        (`TextRenderComponent.K2_SetText` (`self.TextRender`) (`|GetArrayItem` _output_get_2))
        (goto _label))
      (:`Comenzar`
        (if (`self.isCountingDown`)
          ;[0.0625 0.0625 0.0625] Pause
          (`self.StopTimer`)
          (else
            ;[0.05729 0.05729 0.05729] Start timer and notificate if ok or not
            (`/Game/AppContent/Blueprints/Micro/Time_Indicator.StartTimer` _time)
            (bind _countdown (`/Game/AppContent/Blueprints/Micro/Time_Indicator.IsCountingDown` _time))
            (bind _output_get_3 (set `self.isCountingDown` _countdown))
            (set `/Game/AppContent/Blueprints/Micro/Power_Indicator.isCountingDown` _output_get_3 (`self.Power`))))))))

(fn `backToMainMenu`
  (bind _output_get (set `self.ActualMenu` (`self.MainMenu`)))
  (bind _output_get_2 (set `self.index` (`self.mainMenuIndex`)))
  (`TextRenderComponent.K2_SetText` (`self.TextRender`) (`|GetArrayItem` _output_get _output_get_2))
  (set `self.isInSubmenu` false)
  (`self.ChangeMenu`))

(fn `ChangeMenu`
  (bind _output (`|GetArrayItem` (`self.ActualMenu`) (`self.index`)))
  (bind _returnvalue (`KismetTextLibrary.Conv_TextToString` _output))
  (if (`self.isCountingDown`)
    _
    (elif (`self.Encendido`)
      (bind _output_get (set `self.index` (+ (`self.index`) 1)))
      (if (>= _output_get (`KismetArrayLibrary.Array_Length` (`self.ActualMenu`)))
        (set `self.index` 0))
      (if (not (`self.isInSubmenu`))
        (set `self.mainMenuIndex` (`self.index`)))
      (`TextRenderComponent.K2_SetText` (`self.TextRender`) _output)
      (if (or (`KismetStringLibrary.EqualEqual_StrStr` _returnvalue (`KismetTextLibrary.Conv_TextToString` (`|FormatText` "Tiempo"))) (`KismetStringLibrary.EqualEqual_StrStr` _returnvalue (`KismetTextLibrary.Conv_TextToString` (`|FormatText` "Potencia"))))
        (`/Game/AppContent/Blueprints/Micro/RoundSlider.SetIndicator` (`self.Wheel`) (`|GetArrayItem` (`self.ActualMenu`) (`self.index`)))))))

(fn `getActualMenu`
  (returns (AcutalMenu :type "Array of Text"))
  (return (`self.ActualMenu`)))

(fn `isON`
  (returns (NewParam :type Boolean))
  (return (`self.Encendido`)))

(fn `NotificateStop`
  (bind _output_get (set `self.isCountingDown` false))
  (set `/Game/AppContent/Blueprints/Micro/Power_Indicator.isCountingDown` _output_get (`self.Power`)))

(fn `Power Off`
  (`SceneComponent.SetVisibility` (`self.TextRender`) false false)
  (set `self.isCountingDown` false)
  (set `self.Encendido` false)
  ;[0.04167 0.04167 0.04167] Reset the screen
  (set `self.ActualMenu` (`self.MainMenu`))
  (set `self.index` 0)
  (`TextRenderComponent.K2_SetText` (`self.TextRender`) (`|GetArrayItem` (`self.ActualMenu`)))
  (`self.NotificateStop`))

(fn `Power On`
  (`SceneComponent.SetVisibility` (`self.TextRender`) true false)
  (set `self.Encendido` true))

(fn `StopTimer`
  (`/Game/AppContent/Blueprints/Micro/Time_Indicator.StopTimer` (`self.Time`))
  (`self.NotificateStop`))

(fn `useMenuSelector`
  ;[0.0625 0.0625 0.0625] if the time is running then do nothing
  (if (`self.isCountingDown`)
    _
    (elif (`self.isInSubmenu`)
      (`self.backToMainMenu`)
      (else
        (`self.ChangeMenu`)))))

(fn `UserConstructionScript`)