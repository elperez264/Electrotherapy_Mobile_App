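; MicroondasMachine is a microwave actor that assembles its control panel from child actors and links them together on BeginPlay.
; It casts and caches the switch, power and time indicators, round slider, enter button, menu selector, screen and notification manager.
; It then injects cross-references: selector and button get the screen, slider gets both indicators, and switch, time indicator and screen get the notification manager, among others.
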(event `self.ReceiveBeginPlay`
  (`self.Initialize Variables`)
  (`self.Initialize switch`)
  (`self.Initialize Selector`)
  (`self.Initialize EnterButton`)
  (`self.Initialize RoundSlider`)
  (`self.Initialize TimeIndicator`)
  (`self.Initialize Screen`))

(fn `Initialize EnterButton`
  (set `/Game/AppContent/Blueprints/Micro/EnterButton.Pantalla_Menu` (`self.As Menu Micro`) (`self.As Enter Button`)))

(fn `Initialize RoundSlider`
  (bind _as_round_slider (`self.As Round Slider`))
  (set `/Game/AppContent/Blueprints/Micro/RoundSlider.PowerInd` (`self.As Power Indicator`) _as_round_slider)
  (set `/Game/AppContent/Blueprints/Micro/RoundSlider.TImeInd` (`self.As Time Indicator`) _as_round_slider))

(fn `Initialize Screen`
  (bind _as_menu_micro (`self.As Menu Micro`))
  (set `/Game/AppContent/Blueprints/Micro/MenuMicro.Wheel` (`self.As Round Slider`) _as_menu_micro)
  (set `/Game/AppContent/Blueprints/Micro/MenuMicro.UI` (`self.As Notification Manager`) _as_menu_micro)
  (set `/Game/AppContent/Blueprints/Micro/MenuMicro.Time` (`self.As Time Indicator`) _as_menu_micro))

(fn `Initialize Selector`
  (set `/Game/AppContent/Blueprints/Micro/MenuSelector.Pantalla` (`self.As Menu Micro`) (`self.As Menu Selector`)))

(fn `Initialize switch`
  (bind _as_switch (`self.As Switch`))
  (set `/Game/AppContent/Blueprints/Micro/Switch.Power` (`self.As Power Indicator`) _as_switch)
  (set `/Game/AppContent/Blueprints/Micro/Switch.Time` (`self.As Time Indicator`) _as_switch)
  (set `/Game/AppContent/Blueprints/Micro/Switch.Pantalla` (`self.As Menu Micro`) _as_switch)
  (set `/Game/AppContent/Blueprints/Micro/Switch.Notificaciones` (`self.As Notification Manager`) _as_switch))

(fn `Initialize TimeIndicator`
  (set `/Game/AppContent/Blueprints/Micro/Time_Indicator.NotificationManager` (`self.As Notification Manager`) (`self.As Time Indicator`)))

(fn `Initialize Variables`
  (bind _asswitch (cast `/Game/AppContent/Blueprints/Micro/Switch` (`ChildActorComponent.ChildActor` (`self.Switch`))))
  (set `self.As Switch` _asswitch)
  (bind _aspower_indicator (cast `/Game/AppContent/Blueprints/Micro/Power_Indicator` (`ChildActorComponent.ChildActor` (`self.Power_Indicator`))))
  (set `self.As Power Indicator` _aspower_indicator)
  (bind _astime_indicator (cast `/Game/AppContent/Blueprints/Micro/Time_Indicator` (`ChildActorComponent.ChildActor` (`self.Time_Indicator`))))
  (set `self.As Time Indicator` _astime_indicator)
  (bind _asround_slider (cast `/Game/AppContent/Blueprints/Micro/RoundSlider` (`ChildActorComponent.ChildActor` (`self.RoundSlider`))))
  (set `self.As Round Slider` _asround_slider)
  (bind _asenter_button (cast `/Game/AppContent/Blueprints/Micro/EnterButton` (`ChildActorComponent.ChildActor` (`self.EnterButton`))))
  (set `self.As Enter Button` _asenter_button)
  (bind _asmenu_micro (cast `/Game/AppContent/Blueprints/Micro/MenuMicro` (`ChildActorComponent.ChildActor` (`self.Menu`))))
  (set `self.As Menu Micro` _asmenu_micro)
  (bind _asmenu_selector (cast `/Game/AppContent/Blueprints/Micro/MenuSelector` (`ChildActorComponent.ChildActor` (`self.MenuSelector`))))
  (set `self.As Menu Selector` _asmenu_selector)
  (bind _asnotification_manager (cast `/Game/AppContent/Blueprints/NotificationManager` (`ChildActorComponent.ChildActor` (`self.NotificationManager`))))
  (set `self.As Notification Manager` _asnotification_manager))

(fn `UserConstructionScript`)