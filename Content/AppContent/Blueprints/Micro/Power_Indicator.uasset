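; Three-digit power display for the Micro device that stores an adjustable power value and shows it on three text renders.
; Increase and Decrease events step the value only while powered on and not counting down, splitting it into zero-padded characters for the display.
; PowerOn reveals the digits, while PowerOff hides and resets them.
; GetPower, IsMax and IsMin expose the value and its limits, which the step functions do not enforce.
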(event `/Game/AppContent/Interface/IndicatorInterface.Increase`
  (`self.IncreaseValue`))

(event `/Game/AppContent/Interface/IndicatorInterface.Decrease`
  (`self.DecreaseValue`))

(fn `DecreaseValue`
  (bind _returnvalue (+ -1 (`self.Value`)))
  (if (and (`self.Encendido`) (not (`self.isCountingDown`)))
    (set `self.Value` _returnvalue)
    (bind (_first _second _third) (`self.GetNumbers` (`KismetStringLibrary.Conv_IntToString` _returnvalue)))
    (`self.SetNumbers` _first _second _third)))

(fn `GetNumbers`
  (params (Input :type String))
  (returns (First :type String) (Second :type String) (Third :type String))
  (bind _returnvalue (`KismetStringLibrary.GetCharacterArrayFromString` Input))
  (bind _output (`|GetArrayItem` _returnvalue))
  (bind _output_2 (`|GetArrayItem` _returnvalue 1))
  (switch `int` (`KismetArrayLibrary.Array_Length` _returnvalue)
    (:`1`
      (set `self.First` "0")
      (set `self.Second` "0")
      (set `self.Third` _output))
    (:`2`
      (set `self.First` "0")
      (set `self.Second` _output)
      (set `self.Third` _output_2))
    (:`3`
      (set `self.First` _output)
      (set `self.Second` _output_2)
      (set `self.Third` (`|GetArrayItem` _returnvalue 2))))
  (return (`self.First`) (`self.Second`) (`self.Third`)))

(fn `GetPower`
  (returns (value :type Integer))
  (return (`self.Value`)))

(fn `IncreaseValue`
  (bind _returnvalue (+ 1 (`self.Value`)))
  ;[0.0625 0.0625 0.0625] cant be off or the time running
  (if (and (`self.Encendido`) (not (`self.isCountingDown`)))
    (set `self.Value` _returnvalue)
    (bind (_first _second _third) (`self.GetNumbers` (`KismetStringLibrary.Conv_IntToString` _returnvalue)))
    (`self.SetNumbers` _first _second _third)))

(fn `isMax`
  (returns (yes :type Boolean))
  (return (>= (`self.Value`) 349)))

(fn `isMin`
  (returns (yes :type Boolean))
  (return (<= (`self.Value`) 1)))

(fn `Power Off`
  (`SceneComponent.SetVisibility` (`self.TextRender`) false false)
  (`SceneComponent.SetVisibility` (`self.TextRender2`) false false)
  (`SceneComponent.SetVisibility` (`self.TextRender3`) false false)
  (set `self.Encendido` false)
  (`self.SetNumbers` "0" "0" "0")
  (set `self.Value` 0))

(fn `Power On`
  (`SceneComponent.SetVisibility` (`self.TextRender`) true false)
  (`SceneComponent.SetVisibility` (`self.TextRender2`) true false)
  (`SceneComponent.SetVisibility` (`self.TextRender3`) true false)
  (set `self.Encendido` true))

(fn `SetNumbers`
  (params (First :type String) (Second :type String) (Third :type String))
  (`TextRenderComponent.K2_SetText` (`self.TextRender`) (`KismetTextLibrary.Conv_StringToText` First))
  (`TextRenderComponent.K2_SetText` (`self.TextRender2`) (`KismetTextLibrary.Conv_StringToText` Second))
  (`TextRenderComponent.K2_SetText` (`self.TextRender3`) (`KismetTextLibrary.Conv_StringToText` Third)))

(fn `UserConstructionScript`)