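; MenuMicro is an actor that runs the text-screen menu of a simulated device with applicator, emission, time and power options.
; ChangeMenu cycles entries on a TextRender, setting the Wheel's indicator for "Tiempo" or "Potencia".
; Enter switches on the entry's text to open submenus, start the timer and UI via "Comenzar", or otherwise return to the main menu.
; Power functions gate input and visibility; powering off resets the menu and notifies the UI.
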(event `self.ReceiveBeginPlay`
  (set `self.ActualMenu` (`self.MainMenu`)))

(event `/Game/AppContent/Interface/PantallaMenu.Enter`
  (if (`self.Encendido`)
    (switch `string` (`KismetTextLibrary.Conv_TextToString` (`|GetArrayItem` (`self.ActualMenu`) (`self.index`)))
      (:`Default`
        (bind _output_get (set `self.ActualMenu` (`self.MainMenu`)))
        (`TextRenderComponent.K2_SetText` (`self.TextRender`) (`|GetArrayItem` _output_get))
        (set `self.index` 0 :!label _label))
      (:`Tipo de Aplicador`
        (bind _output_get_2 (set `self.ActualMenu` (`self.AplicadorMenu`)))
        (`TextRenderComponent.K2_SetText` (`self.TextRender`) (`|GetArrayItem` _output_get_2))
        (goto _label))
      (:`Tipo de Emision`
        (bind _output_get_3 (set `self.ActualMenu` (`self.EmisionMenu`)))
        (`TextRenderComponent.K2_SetText` (`self.TextRender`) (`|GetArrayItem` _output_get_3))
        (goto _label))
      (:`Comenzar`
        (`/Game/AppContent/Blueprints/Micro/Time_Indicator.StartTimer` (`self.Time`))
        (`/Game/AppContent/Blueprints/NotificationManager.Empezar` (`self.UI`))))))

(fn `ChangeMenu`
  (bind _output (`|GetArrayItem` (`self.ActualMenu`) (`self.index`)))
  (bind _returnvalue (`KismetTextLibrary.Conv_TextToString` _output))
  (if (`self.Encendido`)
    (bind _output_get (set `self.index` (+ (`self.index`) 1)))
    (if (>= _output_get (`KismetArrayLibrary.Array_Length` (`self.ActualMenu`)))
      (set `self.index` 0))
    (`TextRenderComponent.K2_SetText` (`self.TextRender`) _output)
    (if (or (`KismetStringLibrary.EqualEqual_StrStr` _returnvalue (`KismetTextLibrary.Conv_TextToString` (`|FormatText` "Tiempo"))) (`KismetStringLibrary.EqualEqual_StrStr` _returnvalue (`KismetTextLibrary.Conv_TextToString` (`|FormatText` "Potencia"))))
      (`/Game/AppContent/Blueprints/Micro/RoundSlider.SetIndicator` (`self.Wheel`) (`|GetArrayItem` (`self.ActualMenu`) (`self.index`))))))

(fn `getActualMenu`
  (returns (AcutalMenu :type "Array of Text"))
  (return (`self.ActualMenu`)))

(fn `isON`
  (returns (NewParam :type Boolean))
  (return (`self.Encendido`)))

(fn `Power Off`
  (`SceneComponent.SetVisibility` (`self.TextRender`) false false)
  (set `self.Encendido` false)
  ;[0.04167 0.04167 0.04167] Reset the screen
  (set `self.ActualMenu` (`self.MainMenu`))
  (set `self.index` 0)
  (`TextRenderComponent.K2_SetText` (`self.TextRender`) (`|GetArrayItem` (`self.ActualMenu`)))
  (bind _countdown (`/Game/AppContent/Blueprints/Micro/Time_Indicator.IsCountingDown` (`self.Time`)))
  (`/Game/AppContent/Blueprints/NotificationManager.Apagar` (`self.UI`) _countdown))

(fn `Power On`
  (`SceneComponent.SetVisibility` (`self.TextRender`) true false)
  (set `self.Encendido` true))

(fn `UserConstructionScript`)