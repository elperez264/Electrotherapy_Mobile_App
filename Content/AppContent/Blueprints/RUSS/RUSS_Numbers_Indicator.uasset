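; RUSS_Numbers_Indicator is an actor that acts as a numeric display for RUSS pulse, pause, time and two intensity values.
; Its change functions cast the Widget component's user widget to RUSS_Numbers and forward values to the matching set events, with time split into minutes and seconds.
; The max pulse and max pause setters only store their values, and the actor runs no logic of its own on BeginPlay or Tick.
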(fn `ChangeIntensity1`
  (params (NewPercent :type "Float (double-precision)"))
  (bind _asruss_numbers (cast `/Game/AppContent/UI/RUSS_Numbers` (`WidgetComponent.GetUserWidgetObject` (`self.Widget`))))
  (`/Game/AppContent/UI/RUSS_Numbers.SetIntensity_1_Event` _asruss_numbers NewPercent))

(fn `ChangeIntensity2`
  (params (NewPercent :type "Float (double-precision)"))
  (bind _asruss_numbers (cast `/Game/AppContent/UI/RUSS_Numbers` (`WidgetComponent.GetUserWidgetObject` (`self.Widget`))))
  (`/Game/AppContent/UI/RUSS_Numbers.SetIntensity_2_Event` _asruss_numbers NewPercent))

(fn `changePause`
  (params (NewValue :type Integer))
  (bind _asruss_numbers (cast `/Game/AppContent/UI/RUSS_Numbers` (`WidgetComponent.GetUserWidgetObject` (`self.Widget`))))
  (`/Game/AppContent/UI/RUSS_Numbers.SetPause_Event` _asruss_numbers NewValue))

(fn `changePulse`
  (params (newValue :type Integer))
  (bind _asruss_numbers (cast `/Game/AppContent/UI/RUSS_Numbers` (`WidgetComponent.GetUserWidgetObject` (`self.Widget`))))
  (`/Game/AppContent/UI/RUSS_Numbers.SetPulse_Event` _asruss_numbers newValue))

(fn `ChangeTime`
  (params (Seconds :type Integer))
  (bind _asruss_numbers (cast `/Game/AppContent/UI/RUSS_Numbers` (`WidgetComponent.GetUserWidgetObject` (`self.Widget`))))
  (`/Game/AppContent/UI/RUSS_Numbers.SetTime_Event` _asruss_numbers (/ Seconds 60) (mod Seconds 60)))

(fn `setMaxPause`
  (params (NewValue :type "Float (double-precision)"))
  (set `self.MaxPause` NewValue))

(fn `setMaxPulse`
  (params (NewValue :type "Float (double-precision)"))
  (set `self.MaxPulse` NewValue))

(fn `UserConstructionScript`)