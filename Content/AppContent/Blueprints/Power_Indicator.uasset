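; Power_Indicator is an actor Blueprint that displays a numeric power reading on a TextRender component.
; Increase and Decrease step the stored Value up or down by a fixed five and update the text.
; Each function reapplies the step to the updated Value for SetText, so the displayed number lands one step beyond the stored one.
; It has no active event or construction logic, so changes depend on external calls.
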(fn `Decrease`
  (bind _returnvalue (+ -5 (`self.Value`)))
  (set `self.Value` _returnvalue)
  (`TextRenderComponent.K2_SetText` (`self.TextRender`) (`KismetTextLibrary.Conv_IntToText` _returnvalue)))

(fn `Increase`
  (bind _returnvalue (+ 5 (`self.Value`)))
  (set `self.Value` _returnvalue)
  (`TextRenderComponent.K2_SetText` (`self.TextRender`) (`KismetTextLibrary.Conv_IntToText` _returnvalue)))

(fn `UserConstructionScript`)