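; Time_Indicator is a two-digit numeric display actor that holds an integer Value, returned through GetPower.
; Increase and Decrease events step Value by one and refresh two TextRender components.
; GetNumbers splits the number string into two characters, zero-padding single digits.
; Power On/Off toggle the text's visibility, while isMax and isMin report the range limits without clamping Value.
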(event `/Game/AppContent/Interface/IndicatorInterface.Decrease`
  (`self.DecreaseValue`))

(event `/Game/AppContent/Interface/IndicatorInterface.Increase`
  (`self.IncreaseValue`))

(fn `DecreaseValue`
  (bind _returnvalue (+ -1 (`self.Value`)))
  (set `self.Value` _returnvalue)
  (bind (_first _second) (`self.GetNumbers` (`KismetStringLibrary.Conv_IntToString` _returnvalue)))
  (`TextRenderComponent.K2_SetText` (`self.TextRender1`) (`KismetTextLibrary.Conv_StringToText` _first))
  (`TextRenderComponent.K2_SetText` (`self.TextRender2`) (`KismetTextLibrary.Conv_StringToText` _second)))

(fn `GetNumbers`
  (params (Input :type String))
  (returns (First :type String) (Second :type String))
  (bind _returnvalue (`KismetStringLibrary.GetCharacterArrayFromString` Input))
  (bind _output (`|GetArrayItem` _returnvalue))
  (switch `int` (`KismetArrayLibrary.Array_Length` _returnvalue)
    (:`1`
      (set `self.First` "0")
      (set `self.Second` _output))
    (:`2`
      (set `self.First` _output)
      (set `self.Second` (`|GetArrayItem` _returnvalue 1))))
  (return (`self.First`) (`self.Second`)))

(fn `GetPower`
  (returns (value :type Integer))
  (return (`self.Value`)))

(fn `IncreaseValue`
  (bind _returnvalue (+ 1 (`self.Value`)))
  (set `self.Value` _returnvalue)
  (bind (_first _second) (`self.GetNumbers` (`KismetStringLibrary.Conv_IntToString` _returnvalue)))
  (`TextRenderComponent.K2_SetText` (`self.TextRender1`) (`KismetTextLibrary.Conv_StringToText` _first))
  (`TextRenderComponent.K2_SetText` (`self.TextRender2`) (`KismetTextLibrary.Conv_StringToText` _second)))

(fn `isMax`
  (returns (yes :type Boolean))
  (return (>= (`self.Value`) 29)))

(fn `isMin`
  (returns (yes :type Boolean))
  (return (<= (`self.Value`) 1)))

(fn `Power Off`
  (`SceneComponent.SetVisibility` (`self.TextRender1`) false false)
  (`SceneComponent.SetVisibility` (`self.TextRender2`) false false))

(fn `Power On`
  (`SceneComponent.SetVisibility` (`self.TextRender1`) true false)
  (`SceneComponent.SetVisibility` (`self.TextRender2`) true false))

(fn `UserConstructionScript`)