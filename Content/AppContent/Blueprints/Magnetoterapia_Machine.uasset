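; Magnetotherapy machine actor assembled from child actors: increase and decrease Gauss controls, a Gauss indicator and a screen (PantallaMagneto).
; On BeginPlay it casts the child actors and passes the indicator reference to both controls and to the screen as its GaussNumber.
; It only does this wiring, with no Gauss logic of its own, and a failed cast skips the remaining links.
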(event `self.ReceiveBeginPlay`
  (bind _childactor (`ChildActorComponent.ChildActor` (`self.MG_Gauss_Indicator`)))
  (bind _asincrease_mg (cast `/Game/AppContent/Blueprints/IncreaseMG` (`ChildActorComponent.ChildActor` (`self.IncreaseGauss`))))
  (set `/Game/AppContent/Blueprints/IncreaseMG.Indicator` _childactor _asincrease_mg)
  (bind _asdecrease_mg (cast `/Game/AppContent/Blueprints/DecreaseMG` (`ChildActorComponent.ChildActor` (`self.DecreaseGauss`))))
  (set `/Game/AppContent/Blueprints/DecreaseMG.Indicator` _childactor _asdecrease_mg)
  (bind _aspantalla_magneto (cast `/Game/AppContent/Blueprints/PantallaMagneto` (`ChildActorComponent.ChildActor` (`self.PantallaMagneto`))))
  (bind _asmg_gauss_indicator (cast `/Game/AppContent/Blueprints/MG_Gauss_Indicator` _childactor))
  (set `/Game/AppContent/Blueprints/PantallaMagneto.GaussNumber` _asmg_gauss_indicator _aspantalla_magneto))

(fn `UserConstructionScript`)