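; In-world screen of a "Corrientes" (currents) device, apparently electrotherapy, for choosing body part and method and setting time, pulse and pause.
; A moving highlight selects the menu row, routing next/previous input to setters that update text, body-part image or child RUSS_Numbers_Indicator.
; Enter toggles a one-second looping countdown that locks numeric edits and informs Notifications.
; PowerOn reveals the screen; PowerOff covers it, stops the countdown and resets everything.
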(event `self.ReceiveBeginPlay`
  (set `self.ActualMenu` (`self.BodyPart`))
  (bind _asruss_numbers_indicator (cast `/Game/AppContent/Blueprints/RUSS_Numbers_Indicator` (`ChildActorComponent.ChildActor` (`self.RUSS_Numbers_Indicator`))))
  (`/Game/AppContent/Blueprints/RUSS_Numbers_Indicator.setMaxPause` _asruss_numbers_indicator 60.0)
  (`/Game/AppContent/Blueprints/RUSS_Numbers_Indicator.setMaxPulse` _asruss_numbers_indicator 60.0))

(event `/Game/AppContent/Interface/PantallaMenu.Enter`
  (bind _notifications (`self.Notifications`))
  ;[0.04167 0.04167 0.04167] If the timer is setted then stop it, if not, started
  (if (`self.isCountingDown`)
    (bind _output_get (set `self.isCountingDown` false))
    (`/Game/AppContent/Blueprints/NotificationManager.SetCountingDown` (`self.Notifications`) _output_get)
    (`KismetSystemLibrary.K2_ClearAndInvalidateTimerHandle` (`self.Timer`))
    (elif (> (`self.TimeValueSeconds`) 0)
      (bind _returnvalue (`KismetSystemLibrary.K2_SetTimer` null "DecreaseOneSecond" 1.0 true))
      (set `self.Timer` _returnvalue)
      (bind _output_get_2 (set `self.isCountingDown` true))
      (`/Game/AppContent/Blueprints/NotificationManager.SetCountingDown` _notifications _output_get_2)
      (`/Game/AppContent/Blueprints/NotificationManager.Empezar` _notifications))))

(fn `ChangeActualMaterial`
  (params (Name :type Text))
  (switch `string` (`KismetTextLibrary.Conv_TextToString` Name)
    (:`Hand`
      (set `self.ActualImage` "/Game/AppContent/Materials/HandTexture.HandTexture"))
    (:`Neck`
      (set `self.ActualImage` "/Game/AppContent/Materials/NeckTexture.NeckTexture"))
    (:`Shoulders`
      (set `self.ActualImage` "/Game/AppContent/Materials/ShouldersTexture.ShouldersTexture"))
    (:`Back`
      (set `self.ActualImage` "/Game/AppContent/Materials/BackTexture.BackTexture"))
    (:`Feet`
      (set `self.ActualImage` "/Game/AppContent/Materials/FeetTexture.FeetTexture"))
    (:`Legs`
      (set `self.ActualImage` "/Game/AppContent/Materials/LegsTexture.LegsTexture"))))

(fn `ChangeActualMenu`
  ;[0.04167 0.04167 0.04167] Set the text of the actual menu
  (set `self.Previous Menu` (`self.ActualMenu`))
  (switch `int` (`self.IndiceMenu`)
    (:`0`
      (set `self.ActualMenu` (`self.BodyPart`)))
    (:`1`
      (set `self.ActualMenu` (`self.Method`))
      (`PrimitiveComponent.SetMaterial` (`self.Image`) 0 (`self.ActualImage`))
      (`SceneComponent.SetVisibility` (`self.RUSS_Numbers_Indicator`) false false))
    (:`2`
      (set `self.ActualMenu` (`self.Time`))
      (`PrimitiveComponent.SetMaterial` (`self.Image`) 0 "/Engine/BasicShapes/BasicShapeMaterial.BasicShapeMaterial")
      (`SceneComponent.SetVisibility` (`self.RUSS_Numbers_Indicator`) true false))
    (:`3`
      (set `self.ActualMenu` (`self.Impulso`)))
    (:`4`
      (set `self.ActualMenu` (`self.Pausa`)))))

(fn `ChangeColor`
  (params (Previous :type "TextRenderComponent Object Reference") (Next :type "TextRenderComponent Object Reference"))
  (locals (NewLocalVar :type "TextRenderActor Object Reference"))
  ;[0.04167 0.04167 0.04167] Set black
  (`TextRenderComponent.SetTextRenderColor` Previous (make `Color` 0))
  ;[0.04167 0.04167 0.04167] Set white
  (`TextRenderComponent.SetTextRenderColor` Next (make `Color` 255 255 255 255)))

(fn `ChangeImage`
  (params (Name :type Text))
  (`self.ChangeActualMaterial` Name)
  (`PrimitiveComponent.SetMaterial` (`self.Image`) 0 (`self.ActualImage`)))

(fn `DecreaseOneSecond`
  (bind _returnvalue (+ (`self.TimeValueSeconds`) -1))
  (if (> _returnvalue -1)
    (set `self.TimeValueSeconds` _returnvalue)
    (bind _asruss_numbers_indicator (cast `/Game/AppContent/Blueprints/RUSS_Numbers_Indicator` (`ChildActorComponent.ChildActor` (`self.RUSS_Numbers_Indicator`))))
    (`/Game/AppContent/Blueprints/RUSS_Numbers_Indicator.ChangeTime` _asruss_numbers_indicator (`self.TimeValueSeconds`))
    (else
      (set `self.isCountingDown` false)
      (`KismetSystemLibrary.K2_ClearAndInvalidateTimerHandle` (`self.Timer`)))))

(fn `DecreasePause`
  (bind _returnvalue (+ (`self.PauseValue`) -1))
  (if (> _returnvalue 4)
    (set `self.PauseValue` _returnvalue)
    (bind _asruss_numbers_indicator (cast `/Game/AppContent/Blueprints/RUSS_Numbers_Indicator` (`ChildActorComponent.ChildActor` (`self.RUSS_Numbers_Indicator`))))
    (`/Game/AppContent/Blueprints/RUSS_Numbers_Indicator.changePause` _asruss_numbers_indicator (`self.PauseValue`))))

(fn `DecreasePulse`
  (bind _returnvalue (+ (`self.PulseValue`) -1))
  (if (> _returnvalue 0)
    (set `self.PulseValue` _returnvalue)
    (bind _asruss_numbers_indicator (cast `/Game/AppContent/Blueprints/RUSS_Numbers_Indicator` (`ChildActorComponent.ChildActor` (`self.RUSS_Numbers_Indicator`))))
    (`/Game/AppContent/Blueprints/RUSS_Numbers_Indicator.changePulse` _asruss_numbers_indicator (`self.PulseValue`))))

(fn `DecreaseTime`
  (bind _returnvalue (+ (`self.TimeValueSeconds`) -300))
  (if (> _returnvalue 299)
    (set `self.TimeValueSeconds` _returnvalue)
    (else
      (set `self.TimeValueSeconds` 300)))
  (bind _asruss_numbers_indicator (cast `/Game/AppContent/Blueprints/RUSS_Numbers_Indicator` (`ChildActorComponent.ChildActor` (`self.RUSS_Numbers_Indicator`))))
  (`/Game/AppContent/Blueprints/RUSS_Numbers_Indicator.ChangeTime` _asruss_numbers_indicator (`self.TimeValueSeconds`)))

(fn `IncreasePause`
  (bind _returnvalue (+ (`self.PauseValue`) 1))
  (if (< _returnvalue 61)
    (set `self.PauseValue` _returnvalue)
    (bind _asruss_numbers_indicator (cast `/Game/AppContent/Blueprints/RUSS_Numbers_Indicator` (`ChildActorComponent.ChildActor` (`self.RUSS_Numbers_Indicator`))))
    (`/Game/AppContent/Blueprints/RUSS_Numbers_Indicator.changePause` _asruss_numbers_indicator (`self.PauseValue`))))

(fn `IncreasePulse`
  (bind _returnvalue (+ (`self.PulseValue`) 1))
  (if (< _returnvalue 61)
    (set `self.PulseValue` _returnvalue)
    (bind _asruss_numbers_indicator (cast `/Game/AppContent/Blueprints/RUSS_Numbers_Indicator` (`ChildActorComponent.ChildActor` (`self.RUSS_Numbers_Indicator`))))
    (`/Game/AppContent/Blueprints/RUSS_Numbers_Indicator.changePulse` _asruss_numbers_indicator (`self.PulseValue`))))

(fn `IncreaseTime`
  (bind _returnvalue (+ (`self.TimeValueSeconds`) 300))
  (if (< _returnvalue 3601)
    (set `self.TimeValueSeconds` _returnvalue)
    (bind _asruss_numbers_indicator (cast `/Game/AppContent/Blueprints/RUSS_Numbers_Indicator` (`ChildActorComponent.ChildActor` (`self.RUSS_Numbers_Indicator`))))
    (`/Game/AppContent/Blueprints/RUSS_Numbers_Indicator.ChangeTime` _asruss_numbers_indicator (`self.TimeValueSeconds`))))

(fn `NextMenu`
  (bind (_selectionposition_x _selectionposition_y _selectionposition_z) (`KismetMathLibrary.BreakVector` (`self.SelectionPosition`)))
  (bind _returnvalue (+ _selectionposition_y 13.0))
  (if (`self.isOn`)
    (if (not (> (`self.IndiceMenu`) 3))
      (`SceneComponent.K2_SetRelativeLocation` (`self.MenuSelection`) (`KismetMathLibrary.MakeVector` _selectionposition_x _returnvalue _selectionposition_z) false false)
      (set `self.SelectionPosition` (`KismetMathLibrary.MakeVector` _selectionposition_x _returnvalue _selectionposition_z))
      (set `self.IndiceMenu` (+ (`self.IndiceMenu`) 1))
      (`self.ChangeActualMenu`)
      (`self.ChangeColor` (`self.Previous Menu`) (`self.ActualMenu`)))))

(fn `NextMethod`
  (bind _returnvalue (+ (`self.IndiceMethods`) 1))
  (if (<= _returnvalue 1)
    (bind _output_get (set `self.IndiceMethods` _returnvalue))
    (`TextRenderComponent.K2_SetText` (`self.MethodIndicator`) (`|GetArrayItem` (`self.Methods`) _output_get))))

(fn `NextOnSelection`
  (if (`self.isOn`)
    (switch `int` (`self.IndiceMenu`)
      (:`0`
        (`self.NextPart`))
      (:`1`
        (`self.NextMethod`))
      (:`2`
        (if (not (`self.isCountingDown`))
          (`self.IncreaseTime`)))
      (:`3`
        (if (not (`self.isCountingDown`))
          (`self.IncreasePulse`)))
      (:`4`
        (if (not (`self.isCountingDown`))
          (`self.IncreasePause`))))))

(fn `NextPart`
  (bind _returnvalue (+ (`self.IndiceParts`) 1))
  (if (<= _returnvalue 5)
    (bind _output_get (set `self.IndiceParts` _returnvalue))
    (bind _output (`|GetArrayItem` (`self.BodyParts`) _output_get))
    (`TextRenderComponent.K2_SetText` (`self.BodyIndicator`) _output)
    (`self.ChangeImage` _output)))

(fn `PowerOff`
  (bind _notifications (`self.Notifications`))
  (`SceneComponent.SetVisibility` (`self.PantallaApagada`) true false)
  (if (`self.isCountingDown`)
    ;[0.04167 0.04167 0.04167] Stop de timer and tell the notification that is off
    (`KismetSystemLibrary.K2_ClearAndInvalidateTimerHandle` (`self.Timer`))
    (bind _output_get (set `self.isCountingDown` false))
    (`/Game/AppContent/Blueprints/NotificationManager.SetCountingDown` _notifications _output_get)
    ;[0.04167 0.04167 0.04167] Is counting down when the button off is pressed
    (`/Game/AppContent/Blueprints/NotificationManager.Apagar` _notifications true))
  ;[0.04167 0.04167 0.04167] Reset all the values and menu to the default value
  (`self.ResetMenu`)
  (`self.ResetMethod`)
  (`self.ResetBodyPart`)
  (`self.ResetTimes`)
  (set `self.isOn` false))

(fn `PowerOn`
  (`SceneComponent.SetVisibility` (`self.PantallaApagada`) false false)
  (set `self.isOn` true))

(fn `PreviousMenu`
  (bind (_selectionposition_x _selectionposition_y _selectionposition_z) (`KismetMathLibrary.BreakVector` (`self.SelectionPosition`)))
  (bind _returnvalue (+ _selectionposition_y -13.0))
  (if (`self.isOn`)
    (if (not (< (`self.IndiceMenu`) 1))
      (`SceneComponent.K2_SetRelativeLocation` (`self.MenuSelection`) (`KismetMathLibrary.MakeVector` _selectionposition_x _returnvalue _selectionposition_z) false false)
      (set `self.SelectionPosition` (`KismetMathLibrary.MakeVector` _selectionposition_x _returnvalue _selectionposition_z))
      (set `self.IndiceMenu` (+ (`self.IndiceMenu`) -1))
      (`self.ChangeActualMenu`)
      (`self.ChangeColor` (`self.Previous Menu`) (`self.ActualMenu`)))))

(fn `PreviousMethod`
  (bind _returnvalue (+ (`self.IndiceMethods`) -1))
  (if (>= _returnvalue 0)
    (bind _output_get (set `self.IndiceMethods` _returnvalue))
    (`TextRenderComponent.K2_SetText` (`self.MethodIndicator`) (`|GetArrayItem` (`self.Methods`) _output_get))))

(fn `PreviousOnSelection`
  (if (`self.isOn`)
    (switch `int` (`self.IndiceMenu`)
      (:`0`
        (`self.PreviousPart`))
      (:`1`
        (`self.PreviousMethod`))
      (:`2`
        (if (not (`self.isCountingDown`))
          (`self.DecreaseTime`)))
      (:`3`
        (if (not (`self.isCountingDown`))
          (`self.DecreasePulse`)))
      (:`4`
        (if (not (`self.isCountingDown`))
          (`self.DecreasePause`))))))

(fn `PreviousPart`
  (bind _returnvalue (+ (`self.IndiceParts`) -1))
  (if (>= _returnvalue 0)
    (bind _output_get (set `self.IndiceParts` _returnvalue))
    (bind _output (`|GetArrayItem` (`self.BodyParts`) _output_get))
    (`TextRenderComponent.K2_SetText` (`self.BodyIndicator`) _output)
    (`self.ChangeImage` _output)))

(fn `ResetBodyPart`
  (bind _output_get (set `self.IndiceParts` 0))
  (bind _output (`|GetArrayItem` (`self.BodyParts`) _output_get))
  (`TextRenderComponent.K2_SetText` (`self.BodyIndicator`) _output)
  (`self.ChangeImage` _output))

(fn `ResetMenu`
  (set `self.IndiceMenu` 0)
  (`self.ChangeActualMenu`)
  (`self.ChangeColor` (`self.Previous Menu`) (`self.ActualMenu`))
  (`SceneComponent.K2_SetRelativeLocation` (`self.MenuSelection`) (`self.InitialPosition`) false false)
  (set `self.SelectionPosition` (`self.InitialPosition`)))

(fn `ResetMethod`
  (bind _output_get (set `self.IndiceMethods` 0))
  (`TextRenderComponent.K2_SetText` (`self.MethodIndicator`) (`|GetArrayItem` (`self.Methods`) _output_get)))

(fn `ResetTimes`
  (`SceneComponent.SetVisibility` (`self.RUSS_Numbers_Indicator`) false false)
  (bind _asruss_numbers_indicator (cast `/Game/AppContent/Blueprints/RUSS_Numbers_Indicator` (`ChildActorComponent.ChildActor` (`self.RUSS_Numbers_Indicator`))))
  (bind _output_get (set `self.TimeValueSeconds` 0))
  (`/Game/AppContent/Blueprints/RUSS_Numbers_Indicator.ChangeTime` _asruss_numbers_indicator _output_get)
  (bind _output_get_2 (set `self.PulseValue` 1))
  (`/Game/AppContent/Blueprints/RUSS_Numbers_Indicator.changePulse` _asruss_numbers_indicator _output_get_2)
  (bind _output_get_3 (set `self.PauseValue` 5))
  (`/Game/AppContent/Blueprints/RUSS_Numbers_Indicator.changePause` _asruss_numbers_indicator _output_get_3))

(fn `UserConstructionScript`
  (bind _output_get (set `self.SelectionPosition` (`SceneComponent.RelativeLocation` (`self.MenuSelection`))))
  (set `self.InitialPosition` _output_get))